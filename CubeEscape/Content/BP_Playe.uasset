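; BP_Playe is a player for what appears to be a five-lane runner, built around a physics Cube.
; A looping timer feeds forward movement input, and Space applies a jump impulse when grounded.
; A and D teleport the Cube between lanes, but only inside Teleport-tagged overlaps.
; Left/Right-tagged overlaps yaw it 90 degrees and clear world-Y velocity, while FloorDetection tracks Ground contact and clears vertical velocity on landing.
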(event `Move`
  (`self.AddMovementInput` (`SceneComponent.GetForwardVector` (`self.Cube`)) 1.0 true))

(event `self.ReceiveBeginPlay`
  (`KismetSystemLibrary.K2_SetTimerDelegate` (delegate `Move`) 0.01 true))

(event `Key|SpaceBar`
  (params (Key :type "Key Structure"))
  (:`Pressed`
    (if (`self.IsGrounded?`)
      (`PrimitiveComponent.AddImpulse` (`self.Cube`) (0.0 0.0 500.0) "None" true)
      (else
        (`KismetSystemLibrary.PrintString` "AHHHH")))))

(event `Key|A`
  (params (Key :type "Key Structure"))
  (bind _cube (`self.Cube`))
  (:`Pressed`
    (if (and (> (`self.LaneTracker`) -2) (`self.CanTeleport`))
      (`SceneComponent.K2_SetWorldLocation` _cube (+ (* (`SceneComponent.GetRightVector` _cube) -200.0) (`SceneComponent.K2_GetComponentLocation` _cube)) false true)
      (bind _output_get (set `self.LaneTracker` (- (`self.LaneTracker`) 1)))
      (`KismetSystemLibrary.PrintString` (`KismetStringLibrary.Conv_IntToString` _output_get)))))

(event `Key|D`
  (params (Key :type "Key Structure"))
  (bind _cube (`self.Cube`))
  (:`Pressed`
    (if (and (`self.CanTeleport`) (< (`self.LaneTracker`) 2))
      (`SceneComponent.K2_SetWorldLocation` _cube (+ (* (`SceneComponent.GetRightVector` _cube) 200.0) (`SceneComponent.K2_GetComponentLocation` _cube)) false true)
      (bind _output_get (set `self.LaneTracker` (+ (`self.LaneTracker`) 1)))
      (`KismetSystemLibrary.PrintString` (`KismetStringLibrary.Conv_IntToString` _output_get)))))

(event `self.ReceiveActorBeginOverlap`
  (params (OtherActor :type "Actor Object Reference"))
  (bind _cube (`self.Cube`))
  (bind _cube_2 (`self.Cube`))
  (bind _cube_3 (`self.Cube`))
  (bind (_relativerotation_roll _relativerotation_pitch _relativerotation_yaw) (`KismetMathLibrary.BreakRotator` (`SceneComponent.RelativeRotation` _cube)))
  (bind (_relativerotation_roll_2 _relativerotation_pitch_2 _relativerotation_yaw_2) (`KismetMathLibrary.BreakRotator` (`SceneComponent.RelativeRotation` _cube)))
  (`|ExecutionSequence`
    (:`then_0`
      (if (`self.ActorHasTag` OtherActor "Left")
        (`SceneComponent.K2_SetRelativeRotation` _cube (`KismetMathLibrary.MakeRotator` _relativerotation_roll _relativerotation_pitch (+ _relativerotation_yaw -90.0)) false false)
        (bind _returnvalue (`PrimitiveComponent.GetPhysicsLinearVelocity` _cube_3 "None"))
        (`PrimitiveComponent.SetAllPhysicsLinearVelocity` _cube_3 (`KismetMathLibrary.MakeVector` (.x _returnvalue) 0.0 (.z _returnvalue)) false)))
    (:`then_1`
      (if (`self.ActorHasTag` OtherActor "Right")
        (`SceneComponent.K2_SetRelativeRotation` _cube (`KismetMathLibrary.MakeRotator` _relativerotation_roll_2 _relativerotation_pitch_2 (+ _relativerotation_yaw_2 90.0)) false false)
        (bind _returnvalue_2 (`PrimitiveComponent.GetPhysicsLinearVelocity` _cube_2 "None"))
        (`PrimitiveComponent.SetAllPhysicsLinearVelocity` _cube_2 (`KismetMathLibrary.MakeVector` (.x _returnvalue_2) 0.0 (.z _returnvalue_2)) false)))
    (:`then_2`
      (if (`self.ActorHasTag` OtherActor "Teleport")
        (set `self.CanTeleport` true)))))

(event `self.FloorDetection.OnComponentBeginOverlap`
  (params (OverlappedComponent :type "PrimitiveComponent Object Reference") (OtherActor :type "Actor Object Reference") (OtherComp :type "PrimitiveComponent Object Reference") (OtherBodyIndex :type Integer) (bFromSweep :type Boolean) (SweepResult :type "HitResult Structure (by ref)"))
  (bind _cube (`self.Cube`))
  (if (`self.ActorHasTag` OtherActor "Ground")
    (set `self.IsGrounded?` true)
    (bind _returnvalue (`PrimitiveComponent.GetPhysicsLinearVelocity` _cube "None"))
    (`PrimitiveComponent.SetAllPhysicsLinearVelocity` _cube (`KismetMathLibrary.MakeVector` (.x _returnvalue) (.y _returnvalue)) false)))

(event `self.FloorDetection.OnComponentEndOverlap`
  (params (OverlappedComponent :type "PrimitiveComponent Object Reference") (OtherActor :type "Actor Object Reference") (OtherComp :type "PrimitiveComponent Object Reference") (OtherBodyIndex :type Integer))
  (if (`self.ActorHasTag` OtherActor "Ground")
    (set `self.IsGrounded?` false)))

(event `self.ReceiveActorEndOverlap`
  (params (OtherActor :type "Actor Object Reference"))
  (if (`self.ActorHasTag` OtherActor "Teleport")
    (set `self.CanTeleport` false)))

(fn `UserConstructionScript`)